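; Player bullet actor that damages enemy NextBots and turrets on contact.
; HitBox overlaps cast to either enemy type and apply DMG, then spawn a Niagara spark at the sphere and destroy the bullet.
; Blocking hits on the sphere print a debug string and share that spark-and-destroy path, while an older explosion emitter is left unconnected.
; BeginPlay also fires an AI pawn prediction request with zero prediction time.
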(event OnComponentBeginOverlap(HitBox)
  (params (OverlappedComponent :type Primitive%20Component%20Object%20Reference) (OtherActor :type Actor%20Object%20Reference) (OtherComp :type Primitive%20Component%20Object%20Reference) (OtherBodyIndex :type Integer) (bFromSweep :type Boolean) (SweepResult :type Hit%20Result%20Structure%20%28by%20ref%29))
  (bind _dmg (Variables|Default|GetDMG))
  (bind _asbp_base_next_bot (Utilities|Casting|CastToBP_BaseNextBot OtherActor)
    (:then
      (Game|Damage|ApplyDamage _asbp_base_next_bot _dmg 0 0))
    (:CastFailed
      (bind _asbp_turret_base (Utilities|Casting|CastToBP_Turret_Base OtherActor))
      (Game|Damage|ApplyDamage _asbp_turret_base _dmg 0 0)))
  (Niagara|SpawnSystematLocation "/Game/StarterContent/Particles/NS_Spark.NS_Spark" (Transformation|GetWorldLocation (Variables|Default|GetSphere)))
  (Actor|DestroyActor))

(event OnComponentHit(Sphere)
  (params (HitComponent :type Primitive%20Component%20Object%20Reference) (OtherActor :type Actor%20Object%20Reference) (OtherComp :type Primitive%20Component%20Object%20Reference) (NormalImpulse :type Vector :default "0, 0, 0") (Hit :type Hit%20Result%20Structure%20%28by%20ref%29))
  (Development|PrintString "Hello")
  (Niagara|SpawnSystematLocation "/Game/StarterContent/Particles/NS_Spark.NS_Spark" (Transformation|GetWorldLocation (Variables|Default|GetSphere)))
  (Actor|DestroyActor))

(event EventBeginPlay
  (Class|AISensePrediction|RequestPawnPredictionEvent 0 0 0.0))

(fn ConstructionScript)