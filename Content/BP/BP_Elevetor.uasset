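; BP_Elevetor is an elevator platform that moves vertically when something overlaps its trigger Box.
; Overlap begin turns TronPlatform2's emission material green and, after a half-second delay, plays a Timeline that lerps the root's Z from its original location to NewLocation.
; Overlap end switches the material to blue and reverses the Timeline after the same delay.
; The construction script caches the root's world location as the origin, which the Timeline applies through SetRelativeLocation.
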(event OnComponentBeginOverlap(Box)
  (params (OverlappedComponent :type Primitive%20Component%20Object%20Reference) (OtherActor :type Actor%20Object%20Reference) (OtherComp :type Primitive%20Component%20Object%20Reference) (OtherBodyIndex :type Integer) (bFromSweep :type Boolean) (SweepResult :type Hit%20Result%20Structure%20%28by%20ref%29))
  (bind _originlocation (Variables|Default|GetOriginLocation))
  (Rendering|Material|SetMaterial (Variables|Default|GetTron_Platform2) 1 "/Game/CustomMat/Emission_Green.Emission_Green")
  (Utilities|FlowControl|Delay 0.5)
  (bind _newtrack_0 (Timeline|Timeline Play)
    (:Update
      (Transformation|SetRelativeLocation (Variables|Default|GetDefaultSceneRoot) (Math|Vector|Lerp(Vector) (Variables|Default|GetOriginLocation) (Math|Vector|MakeVector (.x _originlocation) (.y _originlocation) (Variables|Default|GetNewLocation)) _newtrack_0) false false))))

(event OnComponentEndOverlap(Box)
  (params (OverlappedComponent :type Primitive%20Component%20Object%20Reference) (OtherActor :type Actor%20Object%20Reference) (OtherComp :type Primitive%20Component%20Object%20Reference) (OtherBodyIndex :type Integer))
  (bind _originlocation (Variables|Default|GetOriginLocation))
  (Rendering|Material|SetMaterial (Variables|Default|GetTron_Platform2) 1 "/Game/CustomMat/Emission_Blue1.Emission_Blue1")
  (Utilities|FlowControl|Delay 0.5)
  (bind _newtrack_0 (Timeline|Timeline Reverse)
    (:Update
      (Transformation|SetRelativeLocation (Variables|Default|GetDefaultSceneRoot) (Math|Vector|Lerp(Vector) (Variables|Default|GetOriginLocation) (Math|Vector|MakeVector (.x _originlocation) (.y _originlocation) (Variables|Default|GetNewLocation)) _newtrack_0) false false))))

(fn ConstructionScript
  (Variables|Default|SetOriginLocation (Transformation|GetWorldLocation (Variables|Default|GetDefaultSceneRoot))))