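; Fire stand actor whose fire component, PFire, can be toggled on and off by the player.
; The construction script sets the initial PFire visibility from the FireStage flag.
; Overlapping the box enables input and sets Unlock, which is not read here; leaving disables input.
; The F key and the FireBegin event share one path that prints a debug string and toggles PFire visibility without updating FireStage.
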(event OnComponentBeginOverlap(Box)
  (params (OverlappedComponent :type Primitive%20Component%20Object%20Reference) (OtherActor :type Actor%20Object%20Reference) (OtherComp :type Primitive%20Component%20Object%20Reference) (OtherBodyIndex :type Integer) (bFromSweep :type Boolean) (SweepResult :type Hit%20Result%20Structure%20%28by%20ref%29))
  (Input|EnableInput (Game|GetPlayerController 0))
  (Variables|Default|SetUnlock true))

(event OnComponentEndOverlap(Box)
  (params (OverlappedComponent :type Primitive%20Component%20Object%20Reference) (OtherActor :type Actor%20Object%20Reference) (OtherComp :type Primitive%20Component%20Object%20Reference) (OtherBodyIndex :type Integer))
  (Input|DisableInput (Game|GetPlayerController 0)))

(event Custom|FireBegin
  ;[1 1 1] Custome Event : Fire Begin
  (Development|PrintString "Hello")
  (Rendering|ToggleVisibility (Variables|Default|GetP_Fire) false))

(event EventBeginPlay)

(event Collision|EventActorBeginOverlap
  (params (OtherActor :type Actor%20Object%20Reference)))

(event EventTick
  (params (DeltaSeconds :type Float%20%28single-precision%29)))

(event Input|KeyboardEvents|F
  (params (Key :type Key%20Structure :default "None"))
  ;[1 1 1] Custome Event : Fire Begin
  (:Pressed
    (Development|PrintString "Hello")
    (Rendering|ToggleVisibility (Variables|Default|GetP_Fire) false)))

(fn ConstructionScript
  (bind _p_fire (Variables|Default|GetP_Fire))
  (if (Variables|Default|GetFireStage)
    (Rendering|SetVisibility _p_fire true false)
    (else
      (Rendering|SetVisibility _p_fire false false))))