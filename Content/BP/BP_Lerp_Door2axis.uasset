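; Sliding door Blueprint that moves SMDoor along a two-stage path when something passes the FrontTricker overlap check.
; Chained timelines lerp its relative location from origin to LocStep1, then to a point combining LocStep1.X with ZOffset as Y.
; On end overlap, it waits TimeDelay, then two separate timelines reverse both stages in order.
; OpenDoor and CloseDoor events trigger the same sequences without the overlap check.
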(event OnComponentEndOverlap(FrontTricker)
  (params (OverlappedComponent :type Primitive%20Component%20Object%20Reference) (OtherActor :type Actor%20Object%20Reference) (OtherComp :type Primitive%20Component%20Object%20Reference) (OtherBodyIndex :type Integer))
  (bind _sm_door (Variables|Default|GetSM_Door))
  (bind _locstep1 (Variables|Default|GetLocStep1))
  (if (Variables|Default|GetAsCollision)
    (Utilities|FlowControl|Delay (Variables|Default|GetTimeDelay))
    (bind _speed (Timeline|Timeline_0 ReverseFromEnd)
      (:Update
        (Transformation|SetRelativeLocationAndRotation _sm_door (Math|Vector|Lerp(Vector) _locstep1 (Math|Vector|MakeVector (.X (Math|Vector|BreakVector _locstep1)) (Variables|Default|GetZOffset) 0.0) _speed) "0, 0, 0" false false))
      (:Finished
        (bind _speed_2 (Timeline|Timeline_1 ReverseFromEnd)
          (:Update
            (Transformation|SetRelativeLocationAndRotation _sm_door (Math|Vector|Lerp(Vector) "0, 0, 0" _locstep1 _speed_2) "0, 0, 0" false false)))))))

(event OnComponentBeginOverlap(FrontTricker)
  (params (OverlappedComponent :type Primitive%20Component%20Object%20Reference) (OtherActor :type Actor%20Object%20Reference) (OtherComp :type Primitive%20Component%20Object%20Reference) (OtherBodyIndex :type Integer) (bFromSweep :type Boolean) (SweepResult :type Hit%20Result%20Structure%20%28by%20ref%29))
  (bind _locstep1 (Variables|Default|GetLocStep1))
  (if (Variables|Default|GetAsCollision)
    (bind _speed (Timeline|Timeline PlayFromStart)
      (:Update
        (Transformation|SetRelativeLocationAndRotation (Variables|Default|GetSM_Door) (Math|Vector|Lerp(Vector) "0, 0, 0" _locstep1 _speed) "0, 0, 0" false false))
      (:Finished
        (bind _speed_2 (Timeline|Timeline_Animate_Door PlayFromStart)
          (:Update
            (Transformation|SetRelativeLocationAndRotation (Variables|Default|GetSM_Door) (Math|Vector|Lerp(Vector) _locstep1 (Math|Vector|MakeVector (.X (Math|Vector|BreakVector _locstep1)) (Variables|Default|GetZOffset) 0.0) _speed_2) "0, 0, 0" false false)))))))

(event Custom|OpenDoor
  (bind _locstep1 (Variables|Default|GetLocStep1))
  (bind _speed (Timeline|Timeline PlayFromStart)
    (:Update
      (Transformation|SetRelativeLocationAndRotation (Variables|Default|GetSM_Door) (Math|Vector|Lerp(Vector) "0, 0, 0" _locstep1 _speed) "0, 0, 0" false false))
    (:Finished
      (bind _speed_2 (Timeline|Timeline_Animate_Door PlayFromStart)
        (:Update
          (Transformation|SetRelativeLocationAndRotation (Variables|Default|GetSM_Door) (Math|Vector|Lerp(Vector) _locstep1 (Math|Vector|MakeVector (.X (Math|Vector|BreakVector _locstep1)) (Variables|Default|GetZOffset) 0.0) _speed_2) "0, 0, 0" false false))))))

(event Custom|CloseDoor
  (bind _sm_door (Variables|Default|GetSM_Door))
  (bind _locstep1 (Variables|Default|GetLocStep1))
  (Utilities|FlowControl|Delay (Variables|Default|GetTimeDelay))
  (bind _speed (Timeline|Timeline_0 ReverseFromEnd)
    (:Update
      (Transformation|SetRelativeLocationAndRotation _sm_door (Math|Vector|Lerp(Vector) _locstep1 (Math|Vector|MakeVector (.X (Math|Vector|BreakVector _locstep1)) (Variables|Default|GetZOffset) 0.0) _speed) "0, 0, 0" false false))
    (:Finished
      (bind _speed_2 (Timeline|Timeline_1 ReverseFromEnd)
        (:Update
          (Transformation|SetRelativeLocationAndRotation _sm_door (Math|Vector|Lerp(Vector) "0, 0, 0" _locstep1 _speed_2) "0, 0, 0" false false))))))

(fn ConstructionScript)