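; BP_LightAcitveHit is a trigger-driven spotlight that is switched on while the third-person player character is inside its box volume.
; Box begin and end overlap events, filtered by a cast to BP_ThirdPersonCharacter, set the Active flag and apply it to the SpotLight's visibility.
; The construction script applies the LightColor variable and the initial Active state to the SpotLight.
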(event OnComponentBeginOverlap(Box)
  (params (OverlappedComponent :type Primitive%20Component%20Object%20Reference) (OtherActor :type Actor%20Object%20Reference) (OtherComp :type Primitive%20Component%20Object%20Reference) (OtherBodyIndex :type Integer) (bFromSweep :type Boolean) (SweepResult :type Hit%20Result%20Structure%20%28by%20ref%29))
  (Utilities|Casting|CastToBP_ThirdPersonCharacter OtherActor)
  (Variables|Default|SetActive? true)
  (Rendering|SetVisibility (Variables|Default|GetSpotLight) (Variables|Default|GetActive?) false))

(event OnComponentEndOverlap(Box)
  (params (OverlappedComponent :type Primitive%20Component%20Object%20Reference) (OtherActor :type Actor%20Object%20Reference) (OtherComp :type Primitive%20Component%20Object%20Reference) (OtherBodyIndex :type Integer))
  (Utilities|Casting|CastToBP_ThirdPersonCharacter OtherActor)
  (Variables|Default|SetActive? false)
  (Rendering|SetVisibility (Variables|Default|GetSpotLight) (Variables|Default|GetActive?) false))

(fn ConstructionScript
  (bind _spotlight (Variables|Default|GetSpotLight))
  (Rendering|Components|Light|SetLightColor _spotlight (Variables|Default|GetLight%20Color) true)
  (Rendering|SetVisibility _spotlight (Variables|Default|GetActive?) false))