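; Base enemy bot that chases the player, attacks up close and destroys itself when health runs out.
; AI perception triggers a faster chase, and forgetting the player starts slower roaming between random tagged patrol points.
; Taking damage, or the player leaving TargetCheck, sets a flag that re-issues the chase every Tick.
; TargetCheck overlap loops a timed attack that shows a warning box, then briefly toggles Attackbox collision to apply damage.
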(event OnTargetPerceptionUpdated(AIPerception)
  (params (Actor :type Actor%20Object%20Reference) (Stimulus :type AI%20Stimulus%20Structure))
  ;[1 0.1249 0.1349] Move When See Player
  (bind _asbp_third_person_character (Utilities|Casting|CastToBP_ThirdPersonCharacter Actor))
  (Variables|Default|SetNeedToGoToPlayer false)
  (Variables|/Script/Engine.CharacterMovementComponent|SetMaxWalkSpeed (Variables|Character|GetCharacterMovement) 3.5e+02)
  (AI|AIMoveTo self "0, 0, 0" _asbp_third_person_character 5.0 false))

(event OnTargetPerceptionForgotten(AIPerception)
  (params (Actor :type Actor%20Object%20Reference))
  ;[0.02316 0 1] After AI Forgotten Player
  (Utilities|Casting|CastToBP_ThirdPersonCharacter Actor)
  (Variables|/Script/Engine.CharacterMovementComponent|SetMaxWalkSpeed (Variables|Character|GetCharacterMovement) 2e+02)
  ;[0.06221 0.8096 1] Roaming Part
  (bind _outactors (Actor|GetAllActorswithTag (Variables|Default|GetTagPatronPath) :!label _label))
  (AI|AIMoveTo self "0, 0, 0" (.OutItem (Utilities|Array|Random _outactors)) 5.0 false
    (:OnSuccess
      (Utilities|FlowControl|Delay 1.0)
      (goto _label))))

(event OnComponentBeginOverlap(TargetCheck)
  (params (OverlappedComponent :type Primitive%20Component%20Object%20Reference) (OtherActor :type Actor%20Object%20Reference) (OtherComp :type Primitive%20Component%20Object%20Reference) (OtherBodyIndex :type Integer) (bFromSweep :type Boolean) (SweepResult :type Hit%20Result%20Structure%20%28by%20ref%29))
  ;[1 1 1] OIvelap With TargetCeckBox
  (Utilities|Casting|CastToBP_ThirdPersonCharacter OtherActor)
  ;;[1 0.01528 0] Perform Attack
  (bind _returnvalue (Utilities|Time|SetTimerbyEvent (delegate Custom|PerformAttack) 0.1 true))
  (Variables|Default|SetTimer _returnvalue))

(event OnComponentEndOverlap(TargetCheck)
  (params (OverlappedComponent :type Primitive%20Component%20Object%20Reference) (OtherActor :type Actor%20Object%20Reference) (OtherComp :type Primitive%20Component%20Object%20Reference) (OtherBodyIndex :type Integer))
  (bind _visualattackbox (Variables|Default|GetVisualAttackBox))
  ;[1 1 1] OIvelap With TargetCeckBox
  (Utilities|Casting|CastToBP_ThirdPersonCharacter OtherActor)
  (Utilities|Time|ClearandInvalidateTimerbyHandle (Variables|Default|GetTimer))
  (Rendering|SetVisibility _visualattackbox false false)
  (Rendering|Material|SetMaterial _visualattackbox 0 "/Game/StarterContent/Materials/EnemyAttackMat/M_EnemyAttackBase_Waring.M_EnemyAttackBase_Waring")
  (Variables|Default|SetNeedToGoToPlayer true))

(event OnComponentBeginOverlap(Attackbox)
  (params (OverlappedComponent :type Primitive%20Component%20Object%20Reference) (OtherActor :type Actor%20Object%20Reference) (OtherComp :type Primitive%20Component%20Object%20Reference) (OtherBodyIndex :type Integer) (bFromSweep :type Boolean) (SweepResult :type Hit%20Result%20Structure%20%28by%20ref%29))
  ;[1 1 1] Overlap with AttackBox
  (bind _asbp_third_person_character (Utilities|Casting|CastToBP_ThirdPersonCharacter OtherActor))
  (Game|Damage|ApplyDamage _asbp_third_person_character 1.0 0 0)
  (Development|PrintString "Attack Player"))

(event Custom|OnTargetPerceptionForgotten_Event
  (params (Actor :type Actor%20Object%20Reference))
  ;[1 1 1] Debug Player
  (Development|PrintString (Utilities|String|ToString(Text) (Utilities|Text|FormatText "AI Forgot this {Actor}" Actor)))
  ;[0.06221 0.8096 1] Roaming Part
  (bind _outactors (Actor|GetAllActorswithTag (Variables|Default|GetTagPatronPath) :!label _label))
  (AI|AIMoveTo self "0, 0, 0" (.OutItem (Utilities|Array|Random _outactors)) 5.0 false
    (:OnSuccess
      (Utilities|FlowControl|Delay 1.0)
      (goto _label))))

(event Custom|PerformAttack
  (bind _visualattackbox (Variables|Default|GetVisualAttackBox))
  ;[1 1 1] OIvelap With TargetCeckBox
  ;;[1 0.01528 0] Perform Attack
  (Rendering|SetVisibility _visualattackbox true false)
  (Utilities|FlowControl|Delay 1.0)
  (Rendering|Material|SetMaterial _visualattackbox 0 "/Game/StarterContent/Materials/EnemyAttackMat/M_EnemyAttackBase_PerformAttack.M_EnemyAttackBase_PerformAttack")
  (Collision|SetCollisionEnabled (Variables|Default|GetAttackbox) "QueryOnly")
  (Collision|SetCollisionEnabled (Variables|Default|GetAttackbox) "NoCollision")
  (Utilities|FlowControl|Delay 0.2)
  (Rendering|Material|SetMaterial (Variables|Default|GetVisualAttackBox) 0 "/Game/StarterContent/Materials/EnemyAttackMat/M_EnemyAttackBase_Waring.M_EnemyAttackBase_Waring")
  (Rendering|SetVisibility (Variables|Default|GetVisualAttackBox) false false))

(event Game|Damage|EventAnyDamage
  (params (Damage :type Float%20%28single-precision%29) (DamageType :type Damage%20Type%20Object%20Reference) (InstigatedBy :type Controller%20Object%20Reference) (DamageCauser :type Actor%20Object%20Reference))
  ;[1 1 1] Apply damage
  ;;[1 1 1] Trigger Enemy Run To Player
  (Variables|Default|SetNeedToGoToPlayer true)
  (Variables|/Script/Engine.CharacterMovementComponent|SetMaxWalkSpeed (Variables|Character|GetCharacterMovement) 3.5e+02)
  (bind _output_get (Variables|Default|SetCurrentHP (- (Variables|Default|GetCurrentHP) Damage)))
  (if (<= _output_get 0.0)
    (Actor|DestroyActor)))

(event EventTick
  (params (DeltaSeconds :type Float%20%28single-precision%29))
  (Utilities|FlowControl|Sequence
    (:then_0
      ;[1 1 1] Enemy Run to Playe When got damage
      (if (Variables|Default|GetNeedToGoToPlayer)
        (AI|AIMoveTo self "0, 0, 0" (Variables|Default|GetPlayer) 5.0 false)))
    (:then_1
      ;[1 1 1] Trigger Perform Damage to Player
      (if (Variables|Default|GetShouldAttack)
        (CallFunction|PerformAttack)))))

(event EventBeginPlay
  (Utilities|FlowControl|Sequence
    (:then_0
      (Collision|SetCollisionEnabled (Variables|Default|GetAttackbox) "NoCollision"))
    (:then_1
      (bind _returnvalue (Actor|GetActorOfClass "/Game/ThirdPerson/Blueprints/BP_ThirdPersonCharacter.BP_ThirdPersonCharacter_C"))
      (Variables|Default|SetPlayer _returnvalue))
    (:then_2
      (Rendering|SetVisibility (Variables|Default|GetVisualAttackBox) false false))))

(fn ConstructionScript
  (Utilities|FlowControl|Sequence
    (:then_0
      (bind _returnvalue (Actor|GetActorOfClass "/Game/ThirdPerson/Blueprints/BP_ThirdPersonCharacter.BP_ThirdPersonCharacter_C"))
      (Variables|Default|SetPlayer _returnvalue)
      (Variables|Default|SetCurrentHP (Variables|Default|GetMaxHP)))
    (:then_1
      ;[1 1 1] Hit box
      (Development|SetHiddeninGame (Variables|Default|GetTargetCheck) (not (Variables|Default|GetShowHtiBox)) false)
      (Development|SetHiddeninGame (Variables|Default|GetAttackbox) (not (Variables|Default|GetShowHtiBox)) false))))