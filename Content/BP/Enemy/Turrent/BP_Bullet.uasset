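; Turret bullet that damages the third-person player character and explodes on impact.
; HitBox overlaps with BP_ThirdPersonCharacter apply DMG, then spawn an explosion emitter at the Sphere's location and destroy the bullet; other overlaps are ignored.
; Any Sphere hit prints a debug string and shares the explode-and-destroy path without applying damage.
; BeginPlay also fires an AI pawn prediction request with zero prediction time.
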(event OnComponentBeginOverlap(HitBox)
  (params (OverlappedComponent :type Primitive%20Component%20Object%20Reference) (OtherActor :type Actor%20Object%20Reference) (OtherComp :type Primitive%20Component%20Object%20Reference) (OtherBodyIndex :type Integer) (bFromSweep :type Boolean) (SweepResult :type Hit%20Result%20Structure%20%28by%20ref%29))
  (bind _asbp_third_person_character (Utilities|Casting|CastToBP_ThirdPersonCharacter OtherActor))
  (Game|Damage|ApplyDamage _asbp_third_person_character (Variables|Default|GetDMG) 0 0)
  (Effects|SpawnEmitteratLocation "/Game/StarterContent/Particles/P_Explosion.P_Explosion" (Transformation|GetWorldLocation (Variables|Default|GetSphere)))
  (Actor|DestroyActor))

(event OnComponentHit(Sphere)
  (params (HitComponent :type Primitive%20Component%20Object%20Reference) (OtherActor :type Actor%20Object%20Reference) (OtherComp :type Primitive%20Component%20Object%20Reference) (NormalImpulse :type Vector :default "0, 0, 0") (Hit :type Hit%20Result%20Structure%20%28by%20ref%29))
  (Development|PrintString "Hello")
  (Effects|SpawnEmitteratLocation "/Game/StarterContent/Particles/P_Explosion.P_Explosion" (Transformation|GetWorldLocation (Variables|Default|GetSphere)))
  (Actor|DestroyActor))

(event EventBeginPlay
  (Class|AISensePrediction|RequestPawnPredictionEvent 0 0 0.0))

(fn ConstructionScript)