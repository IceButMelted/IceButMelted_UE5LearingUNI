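; Base enemy turret that turns toward the player character when PawnSensing sees it and fires from two alternating spawn points.
; Each sighting interpolates toward a look-at rotation, applying yaw to the actor and yaw plus clamped pitch to the Tower.
; The same event restarts a short retriggerable delay, whose completion flip-flops actor spawning between the BulletSpawn1 and BulletSpawn2 transforms.
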(event OnSeePawn(PawnSensing)
  (params (Pawn :type Pawn%20Object%20Reference))
  (bind _asbp_third_person_character (Utilities|Casting|CastToBP_ThirdPersonCharacter Pawn))
  (Utilities|FlowControl|Sequence
    (:then_0
      (Transformation|SetWorldRotation (Variables|Default|GetTower) (Math|Rotator|MakeRotator 0.0 (Math|Float|Clamp(Float) (.pitch (Math|Interpolation|RInterpTo (Transformation|GetActorRotation) (Math|Rotator|FindLookatRotation (Transformation|GetActorLocation) (Transformation|GetActorLocation _asbp_third_person_character)) (Utilities|Time|GetWorldDeltaSeconds) (* 2e+01 5.0))) -5e+01 5e+01) (.yaw (Math|Interpolation|RInterpTo (Transformation|GetActorRotation) (Math|Rotator|FindLookatRotation (Transformation|GetActorLocation) (Transformation|GetActorLocation _asbp_third_person_character)) (Utilities|Time|GetWorldDeltaSeconds) (* 2e+01 5.0)))) false false)
      (Transformation|SetActorRotation (Math|Rotator|MakeRotator 0.0 0.0 (.yaw (Math|Interpolation|RInterpTo (Transformation|GetActorRotation) (Math|Rotator|FindLookatRotation (Transformation|GetActorLocation) (Transformation|GetActorLocation _asbp_third_person_character)) (Utilities|Time|GetWorldDeltaSeconds) (* 2e+01 5.0))))))
    (:then_1
      (Utilities|FlowControl|RetriggerableDelay 0.1)
      (Utilities|FlowControl|FlipFlop
        (:A
          (Game|SpawnActorfromClass "/Game/BP/Enemy/Turrent/BP_Bullet.BP_Bullet_C" (Transformation|GetWorldTransform (Variables|Default|GetBulletSpawn1)) "Undefined" "MultiplyWithRoot" 0 0))
        (:B
          (Game|SpawnActorfromClass "/Game/BP/Enemy/Turrent/BP_Bullet.BP_Bullet_C" (Transformation|GetWorldTransform (Variables|Default|GetBulletSpawn2)) "Undefined" "MultiplyWithRoot" 0 0))))))

(fn ConstructionScript)