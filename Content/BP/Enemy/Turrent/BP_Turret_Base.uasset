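; Base enemy turret that detects the third-person player with PawnSensing, tracks them and shoots.
; Each sighting turns the tower and actor toward the player, starts a looping fire timer once and refreshes a retriggerable delay that clears the seen flag.
; Shots spawn BP_Bullet aimed ahead using target velocity and distance; the timer stops once sight lapses.
; Damage reduces HP until the turret is destroyed, and debug cones visualize its sight.
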(event OnSeePawn(PawnSensing)
  (params (Pawn :type Pawn%20Object%20Reference))
  (Variables|Default|SetSee%20Pawn true)
  (bind _asbp_third_person_character (Utilities|Casting|CastToBP_ThirdPersonCharacter Pawn))
  (Variables|Default|Settarget%20Ref _asbp_third_person_character)
  (Utilities|FlowControl|Sequence
    (:then_0
      ;[1 1 1] Rotate "Face" Face to Player
      (Transformation|SetWorldRotation (Variables|Default|GetTower) (Math|Rotator|MakeRotator (.roll (Math|Interpolation|RInterpTo (Transformation|GetActorRotation) (Math|Rotator|FindLookatRotation (Transformation|GetActorLocation) (Transformation|GetActorLocation (Variables|Default|Gettarget%20Ref))) (Utilities|Time|GetWorldDeltaSeconds) (* 2e+01 5.0))) (Math|Float|Clamp(Float) (.pitch (Math|Interpolation|RInterpTo (Transformation|GetActorRotation) (Math|Rotator|FindLookatRotation (Transformation|GetActorLocation) (Transformation|GetActorLocation (Variables|Default|Gettarget%20Ref))) (Utilities|Time|GetWorldDeltaSeconds) (* 2e+01 5.0))) -1.8e+02 1.8e+02) (.yaw (Math|Interpolation|RInterpTo (Transformation|GetActorRotation) (Math|Rotator|FindLookatRotation (Transformation|GetActorLocation) (Transformation|GetActorLocation (Variables|Default|Gettarget%20Ref))) (Utilities|Time|GetWorldDeltaSeconds) (* 2e+01 5.0)))) false false)
      (Transformation|SetActorRotation (Math|Rotator|MakeRotator 0.0 0.0 (.yaw (Math|Interpolation|RInterpTo (Transformation|GetActorRotation) (Math|Rotator|FindLookatRotation (Transformation|GetActorLocation) (Transformation|GetActorLocation (Variables|Default|Gettarget%20Ref))) (Utilities|Time|GetWorldDeltaSeconds) (* 2e+01 5.0))))))
    (:then_2
      (Utilities|FlowControl|DoOnce false
        (:Completed
          (CallFunction|EnableShootPlayer))))
    (:then_3
      (Utilities|FlowControl|RetriggerableDelay 3.0)
      (Variables|Default|SetSee%20Pawn false))))

(event Custom|Shoot%20Player
  (bind _bulletspawndir (Variables|Default|GetBulletSpawnDir))
  (bind _target_ref (Variables|Default|Gettarget%20Ref))
  (bind _returnvalue (Transformation|GetWorldTransform _bulletspawndir))
  ;[1 1 1] Shooting Bellut to player
  (if (Variables|Default|GetSee%20Pawn)
    (Utilities|FlowControl|RetriggerableDelay 0.1)
    (bind _returnvalue_2 (Game|SpawnActorfromClass "/Game/BP/Enemy/Turrent/BP_Bullet.BP_Bullet_C" (Math|Transform|MakeTransform (.location _returnvalue) (Math|Rotator|FindLookatRotation (.location _returnvalue) (+ (Transformation|GetWorldLocation (Variables|/Script/Engine.Actor|GetRootComponent _target_ref)) (* (Transformation|GetVelocity _target_ref) (/ (Transformation|GetDistanceTo _target_ref) (Variables|Default|GetBulletSpd))))) "1.000000,1.000000,1.000000") "Undefined" "MultiplyWithRoot" 0 0))
    (Variables|/Script/Engine.MovementComponent|SetVelocity (Variables|/Game/BP/Enemy/Turrent/BP_Bullet.BP_Bullet_C|GetProjectileMovement _returnvalue_2) (* (Variables|/Script/Engine.MovementComponent|GetVelocity (Variables|/Game/BP/Enemy/Turrent/BP_Bullet.BP_Bullet_C|GetProjectileMovement _returnvalue_2)) (Variables|Default|GetBulletSpd)))
    (else
      (CallFunction|DisableShootPlayer))))

(event Custom|EnableShootPlayer
  ;[1 1 1] Shooting Bellut to player
  (bind _returnvalue (Utilities|Time|SetTimerbyEvent (delegate Custom|Shoot%20Player) 2.0 true))
  (Variables|Default|SetTimerEventShooting _returnvalue))

(event Custom|DisableShootPlayer
  ;[1 1 1] Shooting Bellut to player
  (Utilities|Time|ClearandInvalidateTimerbyHandle (Variables|Default|GetTimerEventShooting))
  (Utilities|FlowControl|DoOnce false) ; enters at Reset
)

(event Game|Damage|EventAnyDamage
  (params (Damage :type Float%20%28single-precision%29) (DamageType :type Damage%20Type%20Object%20Reference) (InstigatedBy :type Controller%20Object%20Reference) (DamageCauser :type Actor%20Object%20Reference))
  ;[1 0 0] Apply Damage
  (bind _output_get (Variables|Default|SetCurrentHP (- (Variables|Default|GetCurrentHP) Damage)))
  (if (<= _output_get 0.0)
    (Actor|DestroyActor)))

(event EventTick
  (params (DeltaSeconds :type Float%20%28single-precision%29))
  (bind _pawnsensing (Variables|Default|GetPawnSensing))
  (bind _tower (Variables|Default|GetTower))
  (bind _peripheralvisionangle (Variables|/Script/AIModule.PawnSensingComponent|GetPeripheralVisionAngle _pawnsensing))
  (Utilities|FlowControl|Sequence
    (:then_0
      (Class|KismetSystemLibrary|DrawDebugConeinDegrees (Transformation|GetWorldLocation _tower) (Math|Vector|GetForwardVector (Transformation|GetWorldRotation _tower)) (Variables|/Script/AIModule.PawnSensingComponent|GetSightRadius _pawnsensing) _peripheralvisionangle _peripheralvisionangle 12 "(R=1.000000,G=0.000000,B=0.013355,A=1.000000)" 0.1 0.0))))

(fn ConstructionScript
  (bind _pawnsensing (Variables|Default|GetPawnSensing))
  (bind _tower (Variables|Default|GetTower))
  (bind _peripheralvisionangle (Variables|/Script/AIModule.PawnSensingComponent|GetPeripheralVisionAngle _pawnsensing))
  (bind _returnvalue (/ _peripheralvisionangle 2.0))
  (Variables|Default|SetCurrentHP (Variables|Default|GetMaxHP))
  (Class|KismetSystemLibrary|DrawDebugConeinDegrees (Transformation|GetWorldLocation _tower) (Math|Vector|GetForwardVector (Transformation|GetWorldRotation _tower)) (Variables|/Script/AIModule.PawnSensingComponent|GetSightRadius _pawnsensing) _returnvalue _returnvalue 12 "(R=1.000000,G=0.000000,B=0.013355,A=1.000000)" 0.1 0.0))