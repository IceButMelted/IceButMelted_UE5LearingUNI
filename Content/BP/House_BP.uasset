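; House Blueprint with a proximity-triggered light switch for six spotlights and a point light.
; Entering the TriggerCheck volume shows a text render and enables player input; leaving hides it and disables input.
; Pressing F reads the point light's visibility and toggles the spotlights one by one with staggered delays, switching the point light last.
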(event OnComponentBeginOverlap(TriggerCheck)
  (params (OverlappedComponent :type Primitive%20Component%20Object%20Reference) (OtherActor :type Actor%20Object%20Reference) (OtherComp :type Primitive%20Component%20Object%20Reference) (OtherBodyIndex :type Integer) (bFromSweep :type Boolean) (SweepResult :type Hit%20Result%20Structure%20%28by%20ref%29))
  (Rendering|SetVisibility (Variables|Default|GetTextRender) true false)
  (Input|EnableInput (Game|GetPlayerController 0)))

(event OnComponentEndOverlap(TriggerCheck)
  (params (OverlappedComponent :type Primitive%20Component%20Object%20Reference) (OtherActor :type Actor%20Object%20Reference) (OtherComp :type Primitive%20Component%20Object%20Reference) (OtherBodyIndex :type Integer))
  (Rendering|SetVisibility (Variables|Default|GetTextRender) false false)
  (Input|DisableInput (Game|GetPlayerController 0)))

(event EventBeginPlay
  (Variables|Default|SetLightUp (Variables|/Script/Engine.SceneComponent|GetbVisible (Variables|Default|GetPointLight))))

(event Input|KeyboardEvents|F
  (params (Key :type Key%20Structure :default "None"))
  (bind _spot1 (Variables|Default|GetSpot1))
  (bind _spot2 (Variables|Default|GetSpot2))
  (bind _spot3 (Variables|Default|GetSpot3))
  (bind _spot4 (Variables|Default|GetSpot4))
  (bind _spot6 (Variables|Default|GetSpot6))
  (bind _spot5 (Variables|Default|GetSpot5))
  (bind _pointlight (Variables|Default|GetPointLight))
  (:Pressed
    (if (Variables|/Script/Engine.SceneComponent|GetbVisible (Variables|Default|GetPointLight))
      (Rendering|SetVisibility _spot1 false false)
      (Utilities|FlowControl|Delay 0.3)
      (Rendering|SetVisibility _spot2 false false)
      (Utilities|FlowControl|Delay 1.0)
      (Rendering|SetVisibility _spot3 false false)
      (Utilities|FlowControl|Delay 0.3)
      (Rendering|SetVisibility _spot4 false false)
      (Utilities|FlowControl|Delay 1.0)
      (Rendering|SetVisibility _spot5 false false)
      (Utilities|FlowControl|Delay 0.3)
      (Rendering|SetVisibility _spot6 false false)
      (Utilities|FlowControl|Delay 0.6)
      (Rendering|SetVisibility _pointlight false false)
      (else
        (Rendering|SetVisibility _spot1 true false)
        (Utilities|FlowControl|Delay 0.3)
        (Rendering|SetVisibility _spot2 true false)
        (Utilities|FlowControl|Delay 1.0)
        (Rendering|SetVisibility _spot3 true false)
        (Utilities|FlowControl|Delay 0.3)
        (Rendering|SetVisibility _spot4 true false)
        (Utilities|FlowControl|Delay 1.0)
        (Rendering|SetVisibility _spot5 true false)
        (Utilities|FlowControl|Delay 0.3)
        (Rendering|SetVisibility _spot6 true false)
        (Utilities|FlowControl|Delay 0.6)
        (Rendering|SetVisibility _pointlight true false)))))

(fn ConstructionScript)