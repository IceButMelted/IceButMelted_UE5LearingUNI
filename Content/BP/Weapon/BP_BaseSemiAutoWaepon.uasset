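; Base Blueprint for semi-automatic weapons, extending a parent weapon class.
; Shoot calls the parent implementation, then, if CanShoot is set, fires a shot trace over Range and clears the flag.
; A one-shot timer using FireRate as the delay calls ResetShot to re-enable shooting, limiting how often shots fire.
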(event Custom|ResetShot
  (Variables|Default|SetCanShoot? true))

(event EventShoot
  (|CallParentFunction)
  (if (Variables|Default|GetCanShoot?)
    (CallFunction|CreateShotTrace (Variables|Default|GetRange))
    (Variables|Default|SetCanShoot? false)
    (Utilities|Time|SetTimerbyEvent (delegate Custom|ResetShot) (Variables|Default|GetFireRate))))

(fn ConstructionScript
  (|CallParentFunction))