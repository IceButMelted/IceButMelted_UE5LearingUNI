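; BP_BaseWeapon is a base hitscan weapon that handles firing, ammo and reloading for BP_ThirdPersonCharacter, with empty Shoot and EndShoot events.
; CreateShotTrace spends ammo, plays muzzle effects and runs a multi-object line trace from the follow camera with random spread.
; Hits up to a pierce limit get sparks, a BP_Bullet_interact actor and damage.
; ReloadWeapon adds one delayed ammo increment per call without reducing reserve ammo.
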(event Custom|CreateShotTrace
  (params (Range :type Float%20%28double-precision%29))
  (bind _shotarrow (Variables|Default|GetShotArrow))
  (bind _fbulletspread (Variables|GunDetail|GetfBulletSpread))
  (bind _player_character (Variables|Default|GetPlayer%20Character))
  (bind _returnvalue (Transformation|GetWorldTransform _shotarrow))
  (bind _returnvalue_2 (* _fbulletspread 1e+03))
  (bind _followcamera (Variables|/Game/ThirdPerson/Blueprints/BP_ThirdPersonCharacter.BP_ThirdPersonCharacter_C|GetFollowCamera _player_character))
  (bind _returnvalue_3 (Transformation|GetWorldLocation _followcamera))
  (bind _returnvalue_4 (* _returnvalue_2 -1.0))
  (bind _output_get (Variables|Ammo|SetCurrentMagAmmo (Math|Integer|Clamp(Integer) (- (Variables|Ammo|GetCurrentMagAmmo) 1) 0 (Variables|Ammo|GetMaxMagAmmo))))
  (Default|UpdateAmmo (Variables|Default|GetPlayer%20Character) _output_get (Variables|Ammo|GetCurrentReserveAmmo))
  (if (not (<= _output_get 0))
    ;[1 0.6188 0.2984] Spawn Particle at gun
    (Niagara|SpawnSystematLocation "/Game/StarterContent/Particles/NS_MuzzleFlash.NS_MuzzleFlash" (.location _returnvalue) (.rotation _returnvalue))
    (Audio|PlaySound2D "/Game/BP/Weapon/LaserBeam002.LaserBeam002" 0.5 1.0 0.0 0 0)
    ;[0.3033 0.2922 1] RayTracing for Hit
    (bind (_outhits _returnvalue_5) (Class|KismetSystemLibrary|LineTraceMultiforObjects _returnvalue_3 (+ (+ _returnvalue_3 (* (Math|Vector|GetForwardVector (Transformation|GetWorldRotation _followcamera)) Range)) (Math|Vector|MakeVector (Math|Random|RandomFloatinRange _returnvalue_4 _returnvalue_2) (Math|Random|RandomFloatinRange _returnvalue_4 _returnvalue_2) (Math|Random|RandomFloatinRange _returnvalue_4 _returnvalue_2))) (Utilities|Array|MakeArray "ObjectTypeQuery3" "ObjectTypeQuery2" "ObjectTypeQuery1") false 0 "None" true))
    ;[1 1 1] Aply Damage
    (if _returnvalue_5
      ;;[1 1 1] Calcualte Precing Bullet through enemy
      (bind (_array_element _array_index) (Utilities|Array|ForEachLoopwithBreak _outhits :!label _label)
        (:LoopBody
          (Variables|Default|SetHit%20Elemet _array_element)
          (if (> _array_index (Variables|GunDetail|GetPrecingThroughCount))
            (goto _label Break)
            (else
              (Niagara|SpawnSystematLocation "/Game/StarterContent/Particles/NS_Spark_Player.NS_Spark_Player" (.Location (Collision|BreakHitResult (Variables|Default|GetHit%20Elemet))))
              (Game|SpawnActorfromClass "/Game/BP/BP_Bullet_interact.BP_Bullet_interact_C" (Math|Transform|MakeTransform (.Location (Collision|BreakHitResult (Variables|Default|GetHit%20Elemet))) "0, 0, 0" "1.000000,1.000000,1.000000") "Undefined" "MultiplyWithRoot" 0 0)
              (Game|Damage|ApplyDamage (.HitActor (Collision|BreakHitResult (Variables|Default|GetHit%20Elemet))) (Variables|GunDetail|GetDamage) 0 0))))))))

(event Custom|Shoot)

(event Custom|EndShoot)

(event Custom|ReloadWeapon
  ;[1 1 1] Reload
  (Utilities|FlowControl|Delay (Variables|Ammo|GetReloadCoolDownPerTick))
  (if (<= (+ (Variables|Ammo|GetReloadAmmonPerTick) (Variables|Ammo|GetCurrentMagAmmo)) (Variables|Ammo|GetMaxMagAmmo))
    (bind _output_get (Variables|Ammo|SetCurrentMagAmmo (+ (Variables|Ammo|GetReloadAmmonPerTick) (Variables|Ammo|GetCurrentMagAmmo))))
    (Default|UpdateAmmo (Variables|Default|GetPlayer%20Character) _output_get (Variables|Ammo|GetCurrentReserveAmmo))))

(event EventBeginPlay
  (bind _asbp_third_person_character (Utilities|Casting|CastToBP_ThirdPersonCharacter (Game|GetPlayerCharacter 0)))
  (Variables|Default|SetPlayer%20Character _asbp_third_person_character))

(fn ConstructionScript)